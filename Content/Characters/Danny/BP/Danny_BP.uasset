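; Danny character Blueprint that handles costume color swaps and actor mirroring.
; BeginPlay creates dynamic materials for the leotard and shoes and enables player input.
; ColorLoaded applies one of five ColorSwap presets from ColorChosen, while debug-style keys and the Special and Attack inputs trigger the first four directly.
; The Mirror event and both Drump press and release flip the actor's Y axis through a matrix mirror of its transform.
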(event `self.ReceiveBeginPlay`
  (bind _skeletalmesh (`self.SkeletalMesh`))
  (bind _returnvalue (`PrimitiveComponent.CreateDynamicMaterialInstance` _skeletalmesh 2 "/Game/Characters/Danny/Material/Dan_Lietard.Dan_Lietard" "Color"))
  (set `self.Lietard_mat` _returnvalue)
  (bind _returnvalue_2 (`PrimitiveComponent.CreateDynamicMaterialInstance` _skeletalmesh 1 "/Game/Characters/Danny/Material/Dan_Shoes.Dan_Shoes" "None"))
  (set `self.Shoes_Mat` _returnvalue_2)
  (`self.EnableInput` (`GameplayStatics.GetPlayerController` 0)))

(event `InputAction|Special`
  (params (Key :type "Key Structure"))
  ;[1 1 1] LietardsMaterialChange
  (:`Pressed`
    (`MaterialInstanceDynamic.SetVectorParameterValue` (`self.Lietard_mat`) "ColorSwap" (struct :`R` 1.0 :`G` 1.0 :`B` 1.0) :!label _label)
    ;[1 1 1] Shoes Material Change
    (`MaterialInstanceDynamic.SetVectorParameterValue` (`self.Shoes_Mat`) "ColorSwap" (struct :`R` 1.0 :`G` 1.0 :`B` 1.0))))

(event `ColorLoaded`
  (bind _lietard_mat (`self.Lietard_mat`))
  (bind _shoes_mat (`self.Shoes_Mat`))
  (bind _colorchosen (`self.ColorChosen`))
  ;[1 1 1] LietardsMaterialChange
  (if (== _colorchosen 1)
    (goto _label)
    (elif (== _colorchosen 2)
      (`MaterialInstanceDynamic.SetVectorParameterValue` _lietard_mat "ColorSwap" (struct :`R` 1.0 :`G` 0.029205 :`A` 1.0) :!label _label_2)
      ;[1 1 1] Shoes Material Change
      (`MaterialInstanceDynamic.SetVectorParameterValue` _shoes_mat "ColorSwap" (struct :`R` 37.0 :`G` 0.029205 :`A` 1.0))
      (elif (== _colorchosen 3)
        (`MaterialInstanceDynamic.SetVectorParameterValue` _lietard_mat "ColorSwap" (struct :`R` 0.035833 :`G` 0.077185 :`B` 0.2 :`A` 1.0) :!label _label_3)
        (`MaterialInstanceDynamic.SetVectorParameterValue` _shoes_mat "ColorSwap" (struct :`R` 0.035833 :`G` 0.077185 :`B` 37.0 :`A` 1.0))
        (elif (== _colorchosen 4)
          (`MaterialInstanceDynamic.SetVectorParameterValue` _lietard_mat "ColorSwap" (struct :`R` 70.0 :`G` 0.5 :`B` 0.5 :`A` 1.0) :!label _label_4)
          (`MaterialInstanceDynamic.SetVectorParameterValue` _shoes_mat "ColorSwap" (struct :`R` 0.6 :`G` 200.0 :`B` 200.0 :`A` 1.0))
          (elif (== _colorchosen 5)
            (`MaterialInstanceDynamic.SetVectorParameterValue` _lietard_mat "ColorSwap" (struct :`R` 45.0 :`G` 45.0 :`B` 45.0 :`A` 1.0))
            (`MaterialInstanceDynamic.SetVectorParameterValue` _shoes_mat "ColorSwap" (struct :`R` 5.0 :`G` 5.0 :`B` 5.0 :`A` 1.0))))))))

(event `Key|E`
  (params (Key :type "Key Structure"))
  ;[1 1 1] LietardsMaterialChange
  (:`Pressed`
    (goto _label)))

(event `Key|F`
  (params (Key :type "Key Structure"))
  ;[1 1 1] LietardsMaterialChange
  (:`Pressed`
    (goto _label_2)))

(event `Key|R`
  (params (Key :type "Key Structure"))
  ;[1 1 1] LietardsMaterialChange
  (:`Pressed`
    (goto _label_3)))

(event `InputAction|Attack`
  (params (Key :type "Key Structure"))
  ;[1 1 1] LietardsMaterialChange
  (:`Pressed`
    (goto _label_4)))

(event `Key|H`
  (params (Key :type "Key Structure"))
  ;[1 1 1] LietardsMaterialChange
  (:`Pressed`
    (goto _label_4)))

(event `Mirror`
  (`self.K2_SetActorTransform` (`KismetMathLibrary.Conv_MatrixToTransform` (`KismetMathLibrary.Matrix_Mirror` (`KismetMathLibrary.Conv_TransformToMatrix` (`self.GetTransform`)) "None" "Y")) :!label _label_5)
  (`self.K2_AddActorWorldRotation` (struct)))

(event `InputAction|Drump`
  (params (Key :type "Key Structure"))
  (:`Pressed`
    (goto _label_5))
  (:`Released`
    (`self.K2_SetActorTransform` (`KismetMathLibrary.Conv_MatrixToTransform` (`KismetMathLibrary.Matrix_Mirror` (`KismetMathLibrary.Conv_TransformToMatrix` (`self.GetTransform`)) "None" "Y")))
    (`self.K2_AddActorWorldRotation` (struct))))

(event `self.ReceiveTick`
  (params (DeltaSeconds :type "Float (single-precision)")))

(fn `UserConstructionScript`)