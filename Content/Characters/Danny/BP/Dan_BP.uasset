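; Dan's fighter Blueprint, implementing his attacks, specials and super in a fighting game on top of a parent character class, using Arin montages.
; Move events play montages, with timelines nudging the capsule along Direction and gravity changes shaping aerial moves.
; Specials feed the player's steam meter and include a hold-or-dud fireball, command grab and hurtbox-swapping counter.
; Steam1 uses time-dilation freeze; dynamic materials apply the chosen color palette.
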(event `InputAction|Special` :consume false :overrideparent false
  (params (Key :type "Key Structure"))
  ;[0.064 0.5552 0.04098] NeutralSpecial
  (:`Pressed`
    (set `self.HoldingSpecial` true))
  (:`Released`
    (set `self.HoldingSpecial` false)))

(event `NeutSpecial`
  (bind _returnvalue (`KismetMathLibrary.MakeTransform` (.location (`SceneComponent.GetSocketTransform` (`self.Mesh`) "Ar_PunchRangeHB_Socket" "RTS_World")) (.rotation (`SceneComponent.GetSocketTransform` (`self.Mesh`) "Ar_PunchRangeHB_Socket" "RTS_World")) (0.3 0.3 0.3)))
  ;[0.064 0.5552 0.04098] NeutralSpecial
  (`self.Meter_Gain` 5.0)
  (`self.PlayAnimMontage` "/Game/Characters/Arin/Animation/Montages/Arin_S_Montage.Arin_S_Montage" 1.8)
  (`KismetSystemLibrary.Delay` 0.25)
  (if (`self.HoldingSpecial`)
    (bind _returnvalue_2 (`|SpawnActorFromClass` "/Game/Characters/Arin/BPs/Arin_Fireball_BP.Arin_Fireball_BP_C" _returnvalue "Undefined" "OverrideRootScale" null null))
    (set `/Game/Characters/Arin/BPs/Arin_Fireball_BP.Dud?` false _returnvalue_2)
    (bind _projectilemovement (`/Game/Characters/Arin/BPs/Arin_Fireball_BP.ProjectileMovement` _returnvalue_2))
    (set `ProjectileMovementComponent.ProjectileGravityScale` 0.0 _projectilemovement)
    (set `MovementComponent.Velocity` (0.0 600.0 0.0) _projectilemovement)
    (else
      (bind _returnvalue_3 (`|SpawnActorFromClass` "/Game/Characters/Arin/BPs/Arin_Fireball_BP.Arin_Fireball_BP_C" _returnvalue "Undefined" "OverrideRootScale" self null))
      (set `/Game/Characters/Arin/BPs/Arin_Fireball_BP.Dud?` true _returnvalue_3)
      (bind _projectilemovement_2 (`/Game/Characters/Arin/BPs/Arin_Fireball_BP.ProjectileMovement` _returnvalue_3))
      (set `ProjectileMovementComponent.ProjectileGravityScale` 1.0 _projectilemovement_2)
      (set `ProjectileMovementComponent.InitialSpeed` 150.0 _projectilemovement_2))))

(event `JA`
  ;[1 0.04539 0.1351] JumpAttack
  (`self.PlayAnimMontage` "/Game/Characters/Arin/Animation/Montages/Arin_JA_Montage.Arin_JA_Montage"))

(event `NeutAttack`
  (bind _capsulecomponent (`self.CapsuleComponent`))
  ;[0.976 0.2695 0.365] Neutral Attack
  (if (not (`self.NeutAttackFollow`))
    (`SceneComponent.K2_SetWorldLocation` _capsulecomponent (+ (`SceneComponent.K2_GetComponentLocation` _capsulecomponent) (* (`KismetMathLibrary.Conv_DoubleToVector` (`self.Direction`)) (0.0 14.0 0.0))) true false)
    (bind _returnvalue (`self.PlayAnimMontage` "/Game/Characters/Arin/Animation/Montages/Arin_A1_Montage.Arin_A1_Montage"))
    (`KismetSystemLibrary.Delay` 0.03)
    (set `self.NeutAttackFollow` true)
    (`KismetSystemLibrary.Delay` _returnvalue)
    (set `self.NeutAttackFollow` false)))

(event `JFA`
  ;[1 0.04539 0.1351] JumpForwardAttack
  (`self.LaunchCharacter` (0.0 0.0 400.0) false true)
  (`self.PlayAnimMontage` "/Game/Characters/Arin/Animation/Montages/Arin_JFA_Montage.Arin_JFA_Montage"))

(event `InputAction|Attack` :consume false :overrideparent false
  (params (Key :type "Key Structure"))
  (bind _capsulecomponent (`self.CapsuleComponent`))
  ;[0.976 0.2695 0.365] Neutral Attack
  (:`Pressed`
    (if (`NavMovementComponent.IsFalling` (`self.CharacterMovement`))
      _
      (elif (`self.NeutAttackFollow`)
        (set `self.NeutAttackFollow` false)
        (`SceneComponent.K2_SetWorldLocation` _capsulecomponent (+ (`SceneComponent.K2_GetComponentLocation` _capsulecomponent) (* (`KismetMathLibrary.Conv_DoubleToVector` (`self.Direction`)) (0.0 40.0 0.0))) true false)
        (bind _returnvalue (`self.PlayAnimMontage` "/Game/Characters/Arin/Animation/Montages/Arin_A2_Montage.Arin_A2_Montage"))
        (`KismetSystemLibrary.Delay` _returnvalue)))))

(event `Forward Special`
  (bind _capsulecomponent (`self.CapsuleComponent`))
  (bind _returnvalue (`SceneComponent.K2_GetComponentLocation` _capsulecomponent))
  ;[0.064 0.5552 0.04098] ForwardSpecial
  (`self.Meter_Gain` 5.0)
  (`self.PlayAnimMontage` "/Game/Characters/Arin/Animation/Montages/Arin_FS1_Montage.Arin_FS1_Montage")
  (bind (_direction _newtrack_1) (`Timeline|Timeline_6` :!via `PlayFromStart` :!label _label)
    (:`Update`
      (`SceneComponent.K2_SetWorldLocation` _capsulecomponent (`KismetMathLibrary.VLerp` _returnvalue (+ _returnvalue (* (`KismetMathLibrary.Conv_DoubleToVector` (`self.Direction`)) (0.0 2.0 0.0))) _newtrack_1) true false))))

(event `self.ReceiveBeginPlay`
  (bind _mesh (`self.Mesh`))
  ;[1 1 1] BeginPlay
  (bind _returnvalue (`PrimitiveComponent.CreateDynamicMaterialInstance` _mesh 2 "/Game/Characters/Danny/Material/Dan_Lietard.Dan_Lietard" "Color"))
  (set `self.Lietard_mat` _returnvalue)
  (bind _returnvalue_2 (`PrimitiveComponent.CreateDynamicMaterialInstance` _mesh 1 "/Game/Characters/Danny/Material/Dan_Shoes.Dan_Shoes" "None"))
  (set `self.Shoes_Mat` _returnvalue_2)
  (`parent.ReceiveBeginPlay`)
  (`PrimitiveComponent.SetCollisionObjectType` (`self.Crouch_Hurtbox`) "ECC_Destructible" :!label _label_2)
  (`PrimitiveComponent.SetCollisionObjectType` (`self.Stand_Hurtbox`) "ECC_GameTraceChannel3")
  (`PrimitiveComponent.SetCollisionObjectType` (`self.Stand_CounterBox`) "ECC_Destructible"))

(event `JUA`
  ;[1 0.04539 0.1351] JumpUpAttack
  (set `CharacterMovementComponent.GravityScale` 3.5 (`self.CharacterMovement`))
  (`self.PlayAnimMontage` "/Game/Characters/Arin/Animation/Montages/Arin_JUA_Montage.Arin_JUA_Montage"))

(event `self.Steam1`
  (bind _charactermovement (`self.CharacterMovement`))
  (bind _capsulecomponent (`self.CapsuleComponent`))
  (bind _capsulecomponent_2 (`self.CapsuleComponent`))
  (bind _returnvalue (`SceneComponent.K2_GetComponentLocation` _capsulecomponent_2))
  (bind _returnvalue_2 (`SceneComponent.K2_GetComponentLocation` _capsulecomponent))
  ;[0 0.2434 1] Steam1_Grounded
  (if (`NavMovementComponent.IsFalling` _charactermovement)
    ;[0 0.2434 1] Steam1_Air
    (`self.LaunchCharacter` (0.0 0.0 0.0) true true)
    (`MovementComponent.StopMovementImmediately` _charactermovement)
    (`GameplayStatics.SetGlobalTimeDilation` 0.1)
    (set `self.CustomTimeDilation` 11.0)
    (bind _returnvalue_3 (`self.PlayAnimMontage` "/Game/Characters/Arin/Animation/Montages/Arin_Steam1_Montage.Arin_Steam1_Montage"))
    (`KismetSystemLibrary.Delay` 0.3)
    (set `self.CustomTimeDilation` 1.0)
    (`GameplayStatics.SetGlobalTimeDilation` 1.0)
    (bind (_direction _newtrack_1) (`Timeline|Timeline_10` :`NewTime` _returnvalue_3 :!via `PlayFromStart`)
      (:`Update`
        (`SceneComponent.K2_SetWorldLocation` _capsulecomponent_2 (`KismetMathLibrary.VLerp` _returnvalue (+ _returnvalue (* (`KismetMathLibrary.Conv_DoubleToVector` (`self.Direction`)) (0.0 3.0 0.0))) _newtrack_1) true false)))
    (else
      (`MovementComponent.StopMovementImmediately` _charactermovement)
      (`GameplayStatics.SetGlobalTimeDilation` 0.1)
      (set `self.CustomTimeDilation` 12.0)
      (bind _returnvalue_4 (`self.PlayAnimMontage` "/Game/Characters/Arin/Animation/Montages/Arin_Steam1_Montage.Arin_Steam1_Montage"))
      (`KismetSystemLibrary.Delay` 0.1)
      (set `self.CustomTimeDilation` 1.0)
      (`GameplayStatics.SetGlobalTimeDilation` 1.0)
      (bind (_direction_2 _newtrack_1_2) (`Timeline|Timeline_5` :`NewTime` _returnvalue_4 :!via `PlayFromStart`)
        (:`Update`
          (`SceneComponent.K2_SetWorldLocation` _capsulecomponent (`KismetMathLibrary.VLerp` _returnvalue_2 (+ _returnvalue_2 (* (`KismetMathLibrary.Conv_DoubleToVector` (`self.Direction`)) (0.0 3.0 0.0))) _newtrack_1_2) true false))))))

(event `ForwardSucceeded`
  (bind _thegrabbed (`self.TheGrabbed`))
  ;[0.064 0.5552 0.04098] ForwardSpecial
  (`|ExecutionSequence`
    (:`then_0`
      (goto _label :!via `Stop`))
    (:`then_1`
      (`MovementComponent.StopMovementImmediately` (`Character.CharacterMovement` _thegrabbed))
      (`self.PlayAnimMontage` "/Game/Characters/Arin/Animation/Montages/Arin_FS2_Montage.Arin_FS2_Montage")
      (`MovementComponent.StopMovementImmediately` (`self.CharacterMovement`))
      (`KismetSystemLibrary.Delay` 0.4)
      (`self.K2_DetachFromActor` _thegrabbed "KeepWorld" "KeepWorld" "KeepWorld")
      (`self.GrabbedCollisionsOn` _thegrabbed)
      (`/Game/GeneralNeeds/Interfaces/Damage_Calc.Damage` _thegrabbed 80.0 "NewEnumerator5" "NewEnumerator1"))))

(event `BackAttack`
  (bind _capsulecomponent (`self.CapsuleComponent`))
  (bind _returnvalue (`SceneComponent.K2_GetComponentLocation` _capsulecomponent))
  ;[0.9427 0.1679 0.2742] BackAttack
  (bind _returnvalue_2 (`self.PlayAnimMontage` "/Game/Characters/Arin/Animation/Montages/Arin_BA_Montage.Arin_BA_Montage"))
  (bind (_direction _newtrack_1) (`Timeline|BA Timeline` :`NewTime` _returnvalue_2 :!via `PlayFromStart`)
    (:`Update`
      (`SceneComponent.K2_SetWorldLocation` _capsulecomponent (`KismetMathLibrary.VLerp` _returnvalue (+ _returnvalue (* (`KismetMathLibrary.Conv_DoubleToVector` (`self.Direction`)) (0.0 5.0 0.0))) _newtrack_1) true false))))

(event `JBA`
  ;[1 0.04539 0.1351] JumpBackAttack
  (`self.PlayAnimMontage` "/Game/Characters/Arin/Animation/Montages/Arin_JBA_Montage.Arin_JBA_Montage"))

(event `self.OnLanded`
  (params (Hit :type "HitResult Structure (by ref)"))
  ;[1 1 1] On_Landed
  (`parent.OnLanded` Hit)
  (`self.landed`)
  (if (`self.KnockedDown`)
    ;[1 1 1] Changing_Collision_Box_On_Crouch
    (`PrimitiveComponent.SetCollisionObjectType` (`self.Crouch_Hurtbox`) "ECC_GameTraceChannel3")
    (`PrimitiveComponent.SetCollisionObjectType` (`self.Stand_Hurtbox`) "ECC_Destructible")
    (else
      (goto _label_2))))

(event `UpSpecial`
  (bind _charactermovement (`self.CharacterMovement`))
  (bind _capsulecomponent (`self.CapsuleComponent`))
  (bind _returnvalue (`SceneComponent.K2_GetComponentLocation` _capsulecomponent))
  ;[0.064 0.5552 0.04098] UpSpecial
  (`self.Meter_Gain` 10.0)
  (`MovementComponent.StopMovementImmediately` _charactermovement)
  (`KismetSystemLibrary.Delay` 0.1)
  (set `CharacterMovementComponent.GravityScale` 0.0 _charactermovement)
  (`MovementComponent.StopMovementImmediately` _charactermovement)
  (bind _returnvalue_2 (`self.PlayAnimMontage` "/Game/Characters/Arin/Animation/Montages/Arin_US_Montage.Arin_US_Montage"))
  (set `self.US_NewLocation` (+ (+ _returnvalue (* (`KismetMathLibrary.Conv_DoubleToVector` (`self.Direction`)) (0.0 35.0 0.0))) (0.0 0.0 200.0)))
  (bind (_direction _newtrack_1) (`Timeline|US_AnimTime` :!via `PlayFromStart`)
    (:`Update`
      (`SceneComponent.K2_SetWorldLocation` _capsulecomponent (`KismetMathLibrary.VLerp` _returnvalue (`self.US_NewLocation`) _newtrack_1) false true)
      (`KismetSystemLibrary.Delay` _returnvalue_2)
      (set `CharacterMovementComponent.GravityScale` 5.0 _charactermovement))))

(event `ForwardAttack`
  ;[0.8677 0.1509 0.2551] ForwardAttack
  (`self.PlayAnimMontage` "/Game/Characters/Arin/Animation/Montages/Arin_FA_Montage.Arin_FA_Montage"))

(event `JDA`
  ;[1 0.04539 0.1351] JumpDownAttack
  (`self.PlayAnimMontage` "/Game/Characters/Arin/Animation/Montages/Arin_JDA_Montage.Arin_JDA_Montage"))

(event `DownSpecial`
  (bind _capsulecomponent (`self.CapsuleComponent`))
  (bind _returnvalue (`SceneComponent.K2_GetComponentLocation` _capsulecomponent))
  ;[0.064 0.5552 0.04098] DownSpecial
  (`self.Meter_Gain` 10.0)
  (`self.PlayAnimMontage` "/Game/Characters/Arin/Animation/Montages/Arin_DS_Montage.Arin_DS_Montage")
  (bind (_direction _newtrack_1) (`Timeline|Timeline_4_0` :!via `PlayFromStart`)
    (:`Update`
      (`SceneComponent.K2_SetWorldLocation` _capsulecomponent (`KismetMathLibrary.VLerp` _returnvalue (+ _returnvalue (* (`KismetMathLibrary.Conv_DoubleToVector` (`self.Direction`)) (0.0 7.0 0.0))) _newtrack_1) true false))))

(event `UpAttack`
  ;[0.8677 0.1509 0.2551] UpAttack
  (`self.PlayAnimMontage` "/Game/Characters/Arin/Animation/Montages/Arin_UA_Montage.Arin_UA_Montage"))

(event `JS`
  (`self.Meter_Gain` 5.0)
  (`KismetSystemLibrary.PrintString` "JumpSpec"))

(event `self.DrumpLaunch`
  (bind _capsulecomponent (`self.CapsuleComponent`))
  (bind _returnvalue (`SceneComponent.K2_GetComponentLocation` _capsulecomponent))
  ;[1 1 1] Drump_Launch
  (`self.StopAnimMontage` null)
  (`self.PlayAnimMontage` "/Game/Characters/Arin/Animation/Montages/Arin_DrumpLauncher_Montage.Arin_DrumpLauncher_Montage")
  (bind (_direction _newtrack_1) (`Timeline|Timeline_1` :!via `PlayFromStart`)
    (:`Update`
      (`SceneComponent.K2_SetWorldLocation` _capsulecomponent (`KismetMathLibrary.VLerp` _returnvalue (+ _returnvalue (* (`KismetMathLibrary.Conv_DoubleToVector` (`self.Direction`)) (0.0 30.0 0.0))) _newtrack_1) true false))))

(event `DownAttack`
  ;[0.8677 0.1509 0.2551] DownAttack
  (`self.PlayAnimMontage` "/Game/Characters/Arin/Animation/Montages/Arin_DA_Montage.Arin_DA_Montage"))

(event `JBS`
  (`self.Meter_Gain` 3.0)
  (`KismetSystemLibrary.PrintString` "JumpForwardSpec"))

(event `BackSpecial`
  ;[0.064 0.5552 0.04098] BackSpecial
  (`PrimitiveComponent.SetCollisionObjectType` (`self.Crouch_Hurtbox`) "ECC_Destructible")
  (`PrimitiveComponent.SetCollisionObjectType` (`self.Stand_Hurtbox`) "ECC_Destructible")
  (`PrimitiveComponent.SetCollisionObjectType` (`self.Stand_CounterBox`) "ECC_GameTraceChannel4")
  (`self.Meter_Gain` 3.0)
  (`self.PlayAnimMontage` "/Game/Characters/Arin/Animation/Montages/Arin_BS1_Montage.Arin_BS1_Montage")
  (`KismetSystemLibrary.Delay` 0.7)
  (`PrimitiveComponent.SetCollisionObjectType` (`self.Crouch_Hurtbox`) "ECC_Destructible")
  (`PrimitiveComponent.SetCollisionObjectType` (`self.Stand_Hurtbox`) "ECC_GameTraceChannel3")
  (`PrimitiveComponent.SetCollisionObjectType` (`self.Stand_CounterBox`) "ECC_Destructible"))

(event `self.Stand_CounterBox.OnComponentBeginOverlap`
  (params (OverlappedComponent :type "PrimitiveComponent Object Reference") (OtherActor :type "Actor Object Reference") (OtherComp :type "PrimitiveComponent Object Reference") (OtherBodyIndex :type Integer) (bFromSweep :type Boolean) (SweepResult :type "HitResult Structure (by ref)"))
  (bind _instigator (`Actor.Instigator` OtherActor))
  ;[0.064 0.5552 0.04098] BackSpecial
  (`|SpawnActorFromClass` "/Game/Stages/Mesh/KO_Screen.KO_Screen_C" (`KismetMathLibrary.MakeTransform` (-780.0 10.0 480.0) (struct :`Pitch` 90.0) (15.0 17.0 15.0)) "Undefined" "OverrideRootScale" null null)
  (set `Actor.CustomTimeDilation` 0.1 _instigator)
  (bind _returnvalue (`self.PlayAnimMontage` "/Game/Characters/Arin/Animation/Montages/Arin_BS2_Montage.Arin_BS2_Montage"))
  (`KismetSystemLibrary.Delay` _returnvalue)
  (set `Actor.CustomTimeDilation` 1.0 _instigator))

(event `JUS`
  (bind _charactermovement (`self.CharacterMovement`))
  (bind _capsulecomponent (`self.CapsuleComponent`))
  (bind _returnvalue (`SceneComponent.K2_GetComponentLocation` _capsulecomponent))
  ;[0.064 0.5552 0.04098] JumpUpSpecial
  (`self.Meter_Gain` 10.0)
  (`MovementComponent.StopMovementImmediately` _charactermovement)
  (`KismetSystemLibrary.Delay` 0.1)
  (set `CharacterMovementComponent.GravityScale` 0.0 _charactermovement)
  (bind _returnvalue_2 (`self.PlayAnimMontage` "/Game/Characters/Arin/Animation/Montages/Arin_US_Montage.Arin_US_Montage"))
  (set `self.US_NewLocation` (+ (+ _returnvalue (* (`KismetMathLibrary.Conv_DoubleToVector` (`self.Direction`)) (0.0 35.0 0.0))) (0.0 0.0 200.0)))
  (bind (_direction _newtrack_1) (`Timeline|Timeline_7` :!via `PlayFromStart`)
    (:`Update`
      (`SceneComponent.K2_SetWorldLocation` _capsulecomponent (`KismetMathLibrary.VLerp` _returnvalue (`self.US_NewLocation`) _newtrack_1) false true)
      (`KismetSystemLibrary.Delay` _returnvalue_2)
      (set `CharacterMovementComponent.GravityScale` 5.0 _charactermovement))))

(event `Grab Succeeded`
  (`self.Grab_Success`))

(event `JDS`
  (bind _charactermovement (`self.CharacterMovement`))
  (bind _capsulecomponent (`self.CapsuleComponent`))
  (bind _returnvalue (`SceneComponent.K2_GetComponentLocation` _capsulecomponent))
  ;[0.064 0.5552 0.04098] JumpDownSpecial
  (`self.Meter_Gain` 10.0)
  (`self.StopAnimMontage` null)
  (set `CharacterMovementComponent.GravityScale` 0.0 _charactermovement)
  (`MovementComponent.StopMovementImmediately` _charactermovement)
  (`KismetSystemLibrary.Delay` 0.1)
  (`self.PlayAnimMontage` "/Game/Characters/Arin/Animation/Montages/Arin_JDS_Montage.Arin_JDS_Montage" 1.0 "Jump")
  (bind (_direction _newtrack_1) (`Timeline|Timeline_8` :!via `PlayFromStart`)
    (:`Update`
      (`SceneComponent.K2_SetWorldLocation` _capsulecomponent (`KismetMathLibrary.VLerp` _returnvalue (+ _returnvalue (* (`KismetMathLibrary.Conv_DoubleToVector` (`self.Direction`)) (0.0 8.0 0.0))) _newtrack_1) true false)
      (`KismetSystemLibrary.Delay` 0.3)
      (set `CharacterMovementComponent.GravityScale` 5.0 _charactermovement))))

(event `LoadColor`
  (bind _lietard_mat (`self.Lietard_mat`))
  (bind _shoes_mat (`self.Shoes_Mat`))
  (bind _colorchosen (`self.ColorChosen`))
  ;[1 1 1] MaterialChange
  (if (== _colorchosen 1)
    ;[1 1 1] Lietard
    (`MaterialInstanceDynamic.SetVectorParameterValue` _lietard_mat "ColorSwap" (struct :`R` 1.0 :`G` 1.0 :`B` 1.0))
    ;[1 1 1] Shoes
    (`MaterialInstanceDynamic.SetVectorParameterValue` _shoes_mat "ColorSwap" (struct :`R` 1.0 :`G` 1.0 :`B` 1.0))
    (elif (== _colorchosen 2)
      (`MaterialInstanceDynamic.SetVectorParameterValue` _lietard_mat "ColorSwap" (struct :`R` 1.0 :`G` 0.029205 :`A` 1.0))
      (`MaterialInstanceDynamic.SetVectorParameterValue` _shoes_mat "ColorSwap" (struct :`R` 37.0 :`G` 0.029205 :`A` 1.0))
      (elif (== _colorchosen 3)
        (`MaterialInstanceDynamic.SetVectorParameterValue` _lietard_mat "ColorSwap" (struct :`R` 0.035833 :`G` 0.077185 :`B` 0.2 :`A` 1.0))
        (`MaterialInstanceDynamic.SetVectorParameterValue` _shoes_mat "ColorSwap" (struct :`R` 0.035833 :`G` 0.077185 :`B` 37.0 :`A` 1.0))
        (elif (== _colorchosen 4)
          (`MaterialInstanceDynamic.SetVectorParameterValue` _lietard_mat "ColorSwap" (struct :`R` 70.0 :`G` 0.5 :`B` 0.5 :`A` 1.0))
          (`MaterialInstanceDynamic.SetVectorParameterValue` _shoes_mat "ColorSwap" (struct :`R` 0.6 :`G` 200.0 :`B` 200.0 :`A` 1.0))
          (elif (== _colorchosen 5)
            (`MaterialInstanceDynamic.SetVectorParameterValue` _lietard_mat "ColorSwap" (struct :`R` 45.0 :`G` 45.0 :`B` 45.0 :`A` 1.0))
            (`MaterialInstanceDynamic.SetVectorParameterValue` _shoes_mat "ColorSwap" (struct :`R` 5.0 :`G` 5.0 :`B` 5.0 :`A` 1.0))))))))

(event `JFS`
  (bind _charactermovement (`self.CharacterMovement`))
  (bind _capsulecomponent (`self.CapsuleComponent`))
  (bind _returnvalue (`SceneComponent.K2_GetComponentLocation` _capsulecomponent))
  ;[0.064 0.5552 0.04098] ForwardSpecial
  (`self.Meter_Gain` 5.0)
  (`self.StopAnimMontage` null)
  (set `CharacterMovementComponent.GravityScale` 0.0 _charactermovement)
  (`MovementComponent.StopMovementImmediately` _charactermovement)
  (`KismetSystemLibrary.Delay` 0.1)
  (bind _returnvalue_2 (`self.PlayAnimMontage` "/Game/Characters/Arin/Animation/Montages/Arin_FS1_Montage.Arin_FS1_Montage"))
  (bind (_direction _newtrack_1) (`Timeline|Timeline_9` :!via `PlayFromStart`)
    (:`Update`
      (`SceneComponent.K2_SetWorldLocation` _capsulecomponent (`KismetMathLibrary.VLerp` _returnvalue (+ _returnvalue (* (`KismetMathLibrary.Conv_DoubleToVector` (`self.Direction`)) (0.0 2.0 0.0))) _newtrack_1) true false)
      (`KismetSystemLibrary.Delay` (- _returnvalue_2 0.3))
      (set `CharacterMovementComponent.GravityScale` 5.0 _charactermovement))))

(fn `Grab_Success`
  (if (== (`self.GetCurrentMontage`) "/Game/Characters/Arin/Animation/Montages/Arin_FS1_Montage.Arin_FS1_Montage")
    (`self.ForwardSucceeded`)))

(fn `landed`
  (`self.StopAnimMontage` null)
  (set `self.MovementOn` true)
  (set `self.AllControlsOn` true)
  (set `self.SpecialsOn` true)
  (set `self.AttacksOn` true)
  (set `self.NeutAttackFollow` false)
  (set `CharacterMovementComponent.GravityScale` 5.0 (`self.CharacterMovement`)))

(fn `Meter_Gain`
  (params (Meter :type "Float (double-precision)"))
  (bind _asggvs_instance (cast `/Game/GeneralNeeds/GGVS_Instance` (`GameplayStatics.GetGameInstance`)))
  (bind _player1_ (`self.IsPlayer1?`))
  (if _player1_
    (set `/Game/GeneralNeeds/GGVS_Instance.P1Steam_Prog` (+ Meter (`/Game/GeneralNeeds/GGVS_Instance.P1Steam_Prog` _asggvs_instance)) _asggvs_instance)
    (else
      (set `/Game/GeneralNeeds/GGVS_Instance.P2Steam_Prog` (+ (`/Game/GeneralNeeds/GGVS_Instance.P2Steam_Prog` _asggvs_instance) Meter) _asggvs_instance))))

(fn `UserConstructionScript`
  (`parent.UserConstructionScript`))