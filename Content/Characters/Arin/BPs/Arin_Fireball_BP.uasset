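; Arin's fireball projectile, which carries an attached HitBox_BP for damage, launch and steam gain, with a shorter active time when flagged Dud.
; Sphere overlaps skip actors instigated by its owner.
; A normal fireball bursts on non-WorldStatic contact and removes its hitbox, while a Dud stops on WorldStatic and spawns two brief, weaker hitboxes before destroying itself.
; DudContiuousFire2, a variant with reversed ground launch, is never called here.
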(event `self.ReceiveBeginPlay`
  (bind _returnvalue (`|SpawnActorFromClass` "/Game/GeneralNeeds/Hitboxes_Hurbox/HitBox_BP.HitBox_BP_C" (`KismetMathLibrary.MakeTransform` (.location (`self.GetTransform` self)) (.rotation (`self.GetTransform` self))) "Undefined" "OverrideRootScale" self (`self.GetInstigator`)))
  (bind _output_get (set `self.Hitbox` _returnvalue))
  (`self.K2_AttachToActor` _output_get self "None" "SnapToTarget" "SnapToTarget" "KeepWorld" true)
  (set `/Game/GeneralNeeds/Hitboxes_Hurbox/HitBox_BP.DamageAmount` 60 _returnvalue)
  (set `/Game/GeneralNeeds/Hitboxes_Hurbox/HitBox_BP.HitHeight` "NewEnumerator1" _returnvalue)
  (set `/Game/GeneralNeeds/Hitboxes_Hurbox/HitBox_BP.HitType` "NewEnumerator1" _returnvalue)
  (set `/Game/GeneralNeeds/Hitboxes_Hurbox/HitBox_BP.Sound` "/Game/Music_SFXs/Voices/Arin/Arin_SmallHit_cue.Arin_SmallHit_cue" _returnvalue)
  (set `/Game/GeneralNeeds/Hitboxes_Hurbox/HitBox_BP.OwnSteamGain` 18.0 _returnvalue)
  (set `/Game/GeneralNeeds/Hitboxes_Hurbox/HitBox_BP.OppSteamGain` 9.0 _returnvalue)
  (set `/Game/GeneralNeeds/Hitboxes_Hurbox/HitBox_BP.Air Launch Distance` (0.0 100.0 100.0) _returnvalue)
  (set `/Game/GeneralNeeds/Hitboxes_Hurbox/HitBox_BP.Ground Launch Distance` (0.0 100.0 20.0) _returnvalue)
  (if (`self.Dud?`)
    (set `/Game/GeneralNeeds/Hitboxes_Hurbox/HitBox_BP.ActiveTime` 1.0 _returnvalue)
    (else
      (set `/Game/GeneralNeeds/Hitboxes_Hurbox/HitBox_BP.ActiveTime` 2.0 _returnvalue))))

(event `self.Sphere.OnComponentBeginOverlap`
  (params (OverlappedComponent :type "PrimitiveComponent Object Reference") (OtherActor :type "Actor Object Reference") (OtherComp :type "PrimitiveComponent Object Reference") (OtherBodyIndex :type Integer) (bFromSweep :type Boolean) (SweepResult :type "HitResult Structure (by ref)"))
  (if (== (`Actor.Instigator` OtherActor) (`self.GetOwner`))
    _
    (elif (`|EnumEquality` (`PrimitiveComponent.GetCollisionObjectType` OtherComp) "ECC_WorldStatic")
      (if (`self.Dud?`)
        (set `ProjectileMovementComponent.ProjectileGravityScale` 0.0 (`self.ProjectileMovement`))
        (`MovementComponent.StopMovementImmediately` (`self.ProjectileMovement`))
        (`ActorComponent.Activate` (`self.InitialBurst_P`) true)
        (`self.DudContiuousFire`)
        (`KismetSystemLibrary.Delay` 0.1)
        (`self.DudContiuousFire`)
        (`KismetSystemLibrary.Delay` 0.1)
        (`self.K2_DestroyActor`))
      (elif (not (`self.Dud?`))
        (`MovementComponent.StopMovementImmediately` (`self.ProjectileMovement`))
        (`ActorComponent.Activate` (`self.InitialBurst_P`) true)
        (`ActorComponent.Deactivate` (`self.laggingFlame`))
        (`SceneComponent.SetVisibility` (`self.Sphere`) false false)
        (`self.K2_DestroyActor` (`self.Hitbox`))
        (`KismetSystemLibrary.Delay` 0.3)
        (`self.K2_DestroyActor`)))))

(fn `DudContiuousFire`
  (bind _returnvalue (`|SpawnActorFromClass` "/Game/GeneralNeeds/Hitboxes_Hurbox/HitBox_BP.HitBox_BP_C" (`KismetMathLibrary.MakeTransform` (.location (`self.GetTransform` self)) (.rotation (`self.GetTransform` self)) (2.0 2.0 2.0)) "Undefined" "OverrideRootScale" self (`self.GetInstigator`)))
  (`self.K2_AttachToActor` _returnvalue self "None" "SnapToTarget" "SnapToTarget" "KeepWorld" true)
  (set `/Game/GeneralNeeds/Hitboxes_Hurbox/HitBox_BP.ActiveTime` 0.1 _returnvalue)
  (set `/Game/GeneralNeeds/Hitboxes_Hurbox/HitBox_BP.DamageAmount` 10 _returnvalue)
  (set `/Game/GeneralNeeds/Hitboxes_Hurbox/HitBox_BP.HitHeight` "NewEnumerator1" _returnvalue)
  (set `/Game/GeneralNeeds/Hitboxes_Hurbox/HitBox_BP.HitType` "NewEnumerator0" _returnvalue)
  (set `/Game/GeneralNeeds/Hitboxes_Hurbox/HitBox_BP.Sound` "/Game/Music_SFXs/Sounds/SmallHit_Cue.SmallHit_Cue" _returnvalue)
  (set `/Game/GeneralNeeds/Hitboxes_Hurbox/HitBox_BP.OwnSteamGain` 5.0 _returnvalue)
  (set `/Game/GeneralNeeds/Hitboxes_Hurbox/HitBox_BP.OppSteamGain` 3.0 _returnvalue)
  (set `/Game/GeneralNeeds/Hitboxes_Hurbox/HitBox_BP.Ground Launch Distance` (0.0 50.0 0.0) _returnvalue)
  (set `/Game/GeneralNeeds/Hitboxes_Hurbox/HitBox_BP.Air Launch Distance` (0.0 100.0 120.0) _returnvalue))

(fn `DudContiuousFire2`
  (bind _returnvalue (`|SpawnActorFromClass` "/Game/GeneralNeeds/Hitboxes_Hurbox/HitBox_BP.HitBox_BP_C" (`KismetMathLibrary.MakeTransform` (.location (`self.GetTransform` self)) (.rotation (`self.GetTransform` self)) (2.0 2.0 2.0)) "Undefined" "OverrideRootScale" self (`self.GetInstigator`)))
  (`self.K2_AttachToActor` _returnvalue self "None" "SnapToTarget" "SnapToTarget" "KeepWorld" true)
  (set `/Game/GeneralNeeds/Hitboxes_Hurbox/HitBox_BP.ActiveTime` 0.1 _returnvalue)
  (set `/Game/GeneralNeeds/Hitboxes_Hurbox/HitBox_BP.DamageAmount` 10 _returnvalue)
  (set `/Game/GeneralNeeds/Hitboxes_Hurbox/HitBox_BP.HitHeight` "NewEnumerator1" _returnvalue)
  (set `/Game/GeneralNeeds/Hitboxes_Hurbox/HitBox_BP.HitType` "NewEnumerator0" _returnvalue)
  (set `/Game/GeneralNeeds/Hitboxes_Hurbox/HitBox_BP.Sound` "/Game/Music_SFXs/Sounds/SmallHit_Cue.SmallHit_Cue" _returnvalue)
  (set `/Game/GeneralNeeds/Hitboxes_Hurbox/HitBox_BP.OwnSteamGain` 5.0 _returnvalue)
  (set `/Game/GeneralNeeds/Hitboxes_Hurbox/HitBox_BP.OppSteamGain` 3.0 _returnvalue)
  (set `/Game/GeneralNeeds/Hitboxes_Hurbox/HitBox_BP.Ground Launch Distance` (0.0 -50.0 0.0) _returnvalue)
  (set `/Game/GeneralNeeds/Hitboxes_Hurbox/HitBox_BP.Air Launch Distance` (0.0 100.0 120.0) _returnvalue))

(fn `UserConstructionScript`)