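; Short-lived fighting-game hitbox actor that despawns after ActiveTime or on the instigator character's destroy event.
; Its first overlap with a vulnerable character other than the instigator plays a sound and sends damage and meter gain through messages.
; It then triggers hit-freeze with an impact particle, flags one hit type's success, and attaches grabbed opponents to the attacker's GrabSocket.
; Combo-based damage scaling exists but is disconnected.
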(event `self.ReceiveBeginPlay`
  (bind _returnvalue (`self.GetOwner`))
  (bind _returnvalue_2 (`self.GetInstigator`))
  (if (not (== _returnvalue (`self.GetInstigatorController`)))
    (set `self.POwner` _returnvalue))
  (set `self.PlayerOwner` _returnvalue_2)
  (set `self.TheSelf` (`self.GetInstigatorController` _returnvalue_2))
  (`KismetSystemLibrary.Delay` 0.005)
  (bind _asbp_grump_parent (cast `/Game/Characters/BP_Grump_Parent` _returnvalue_2)
    (:`then`
      (add `/Game/Characters/BP_Grump_Parent.HitboxDestroy` _asbp_grump_parent (delegate `destroy itself`)))
    (:`CastFailed`
      _))
  (`KismetSystemLibrary.Delay` (`self.ActiveTime`))
  (`self.K2_DestroyActor`))

(event `destroy itself`
  (`self.K2_DestroyActor`))

(event `self.Hitbox_Collision.OnComponentBeginOverlap`
  (params (OverlappedComponent :type "PrimitiveComponent Object Reference") (OtherActor :type "Actor Object Reference") (OtherComp :type "PrimitiveComponent Object Reference") (OtherBodyIndex :type Integer) (bFromSweep :type Boolean) (SweepResult :type "HitResult Structure (by ref)"))
  (if (not (== (`self.PlayerOwner`) OtherActor))
    (set `self.Opponent` OtherActor)
    (bind _asbp_grump_parent (cast `/Game/Characters/BP_Grump_Parent` OtherActor))
    (if (not (`/Game/Characters/BP_Grump_Parent.Invulnerable` _asbp_grump_parent))
      (`/Engine/EditorBlueprintResources/StandardMacros.DoOnce` false
        (:`Completed`
          (`GameplayStatics.PlaySound2D` (`self.Sound`) 0.3 1.0 0.0 null null)
          (bind _asggvs_instance (cast `/Game/GeneralNeeds/GGVS_Instance` (`GameplayStatics.GetGameInstance`)))
          (`KismetSystemLibrary.Delay` 0.02)
          (message `/Game/GeneralNeeds/Interfaces/Damage_Calc.Damage` (`self.Opponent`) (* (`KismetMathLibrary.Conv_IntToDouble` (`self.DamageAmount`)) (`self.DmgScale`)) (`self.HitType`) (`self.HitHeight`) (`self.Ground Launch Distance`) (`self.Air Launch Distance`))
          (message `/Game/GeneralNeeds/Interfaces/MeterGain.MeterGain` (`self.PlayerOwner`) 0.0 (`self.OwnSteamGain`))
          (message `/Game/GeneralNeeds/Interfaces/MeterGain.MeterGain` (`self.Opponent`) (`self.OppSteamGain`) 0.0)
          (`/Engine/EditorBlueprintResources/StandardMacros.DoOnce` false
            (:`Completed`
              (`self.HitFroze`)
              (if (`|EnumEquality` (`self.HitType`) "NewEnumerator3")
                (bind _asbp_grump_parent_2 (cast `/Game/Characters/BP_Grump_Parent` (`self.PlayerOwner`)))
                (set `/Game/Characters/BP_Grump_Parent.DrumpSuccess` true _asbp_grump_parent_2)
                (else
                  ;[1 1 1] Grabbed
                  (if (`|EnumEquality` (`self.HitType`) "NewEnumerator8")
                    (bind _asbp_grump_parent_3 (cast `/Game/Characters/BP_Grump_Parent` (`self.PlayerOwner`)))
                    (if (not (`/Game/Characters/BP_Grump_Parent.Stunned` _asbp_grump_parent_3))
                      (set `/Game/Characters/BP_Grump_Parent.Invulnerable` true _asbp_grump_parent_3)
                      (`/Game/Characters/BP_Grump_Parent.Grab Succeeded` _asbp_grump_parent_3)
                      (bind _asbp_grump_parent_4 (cast `/Game/Characters/BP_Grump_Parent` (`self.Opponent`)))
                      (set `/Game/Characters/BP_Grump_Parent.StunMeter` 99.0 _asbp_grump_parent_4)
                      (set `/Game/Characters/BP_Grump_Parent.TheGrabbed` _asbp_grump_parent_4 _asbp_grump_parent_3)
                      (`/Game/Characters/BP_Grump_Parent.GrabbedCollisionsOff` _asbp_grump_parent_4)
                      (bind _charactermovement (`Character.CharacterMovement` _asbp_grump_parent_4))
                      (set `CharacterMovementComponent.GravityScale` 0.0 _charactermovement)
                      (`MovementComponent.StopMovementImmediately` _charactermovement)
                      (`self.K2_AttachToComponent` _asbp_grump_parent_4 (`Character.Mesh` _asbp_grump_parent_3) (`self.GrabSocket`) "SnapToTarget" "KeepWorld" "KeepWorld" true))
                    (else
                      ;[1 1 1] Special_Launcher
                      (if (`|EnumEquality` (`self.HitType`) "NewEnumerator7")
                        (cast `/Game/Characters/BP_Grump_Parent` (`self.Opponent`))))))))))))))

(event `HitFroze`
  (bind _hittype (`self.HitType`))
  ;[1 1 1] HitFreeze Per Hit
  (`/Engine/EditorBlueprintResources/StandardMacros.IsValid` (`self.POwner`)
    (:`Is Valid`
      _)
    (:`Is Not Valid`
      (bind _asbp_grump_parent (cast `/Game/Characters/BP_Grump_Parent` (`self.PlayerOwner`)))))
  (bind _asbp_grump_parent_2 (cast `/Game/Characters/BP_Grump_Parent` (`self.Opponent`)))
  (`/Game/Characters/BP_Grump_Parent.HitFroze` _asbp_grump_parent _hittype)
  (`/Game/Characters/BP_Grump_Parent.HitFroze` _asbp_grump_parent_2 _hittype)
  (`GameplayStatics.SpawnEmitterAtLocation` "/Game/FXVarietyPack/Particles/P_ky_hit2.P_ky_hit2" (+ (`self.K2_GetActorLocation` self) (-20.0 0.0 0.0)) (struct) (0.5 0.5 0.5)))

(fn `UserConstructionScript`)