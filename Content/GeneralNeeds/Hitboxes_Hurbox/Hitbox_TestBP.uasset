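; Test hitbox actor that follows its owner and prints debug messages on overlaps.
; Each tick it moves its Cube to a fixed X, a Y offset from the owner's location, and the owner's Z.
; Hitbox overlaps print the component name, then ignore actors owned by the same owner.
; A constant-false branch makes the hit-and-destroy path unreachable, so other overlaps print the "just me" message.
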(event `self.ReceiveBeginPlay`
  (set `self.OwningPlayer_Ref` (`self.GetOwner`)))

(event `self.ReceiveTick`
  (params (DeltaSeconds :type "Float (single-precision)"))
  (bind (_returnvalue_x _returnvalue_y _returnvalue_z) (`KismetMathLibrary.BreakVector` (`self.K2_GetActorLocation` (`self.OwningPlayer_Ref`))))
  (`SceneComponent.K2_SetWorldLocation` (`self.Cube`) (`KismetMathLibrary.MakeVector` -870.0 (+ _returnvalue_y 80.0) _returnvalue_z) false false))

(event `self.Hitbox.OnComponentBeginOverlap`
  (params (OverlappedComponent :type "PrimitiveComponent Object Reference") (OtherActor :type "Actor Object Reference") (OtherComp :type "PrimitiveComponent Object Reference") (OtherBodyIndex :type Integer) (bFromSweep :type Boolean) (SweepResult :type "HitResult Structure (by ref)"))
  (`KismetSystemLibrary.PrintString` (`KismetSystemLibrary.GetDisplayName` OverlappedComponent))
  (if (not (== (`self.GetOwner` OtherActor) (`self.OwningPlayer_Ref`)))
    (if false
      (`KismetSystemLibrary.PrintString` "I HAVE BEEN HIT" true true (struct :`R` 1.0 :`B` 0.140353 :`A` 1.0))
      (`self.K2_DestroyActor`)
      (else
        (`KismetSystemLibrary.PrintString` "It's just me dood" true true (struct :`G` 1.0 :`B` 0.08531 :`A` 1.0))))))

(fn `UserConstructionScript`)