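; Music player that plays an intro then crossfades into loop audio, for the menu or a stage.
; The track is chosen by SongIndex, which in stages is a random pick between the two players' indices from GGVS_Instance.
; Playback-percent events near each track's end, gated by DoOnce, fade the intro into MusicLoop, then MusicLoop into MusicLoopB.
; The intro variable is repointed to MusicLoopB after the first handoff.
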(event `self.ReceiveBeginPlay`
  (if (`self.MenuMusic`)
    (bind _output_get (set `self.IntroList` (`|MakeArray` "/Game/Music_SFXs/Menus/MainMenu_BGM_Start.MainMenu_BGM_Start" "/Game/Music_SFXs/Theme/Arin_Theme_Intro.Arin_Theme_Intro" "/Game/Music_SFXs/Theme/DannyTheme_Intro.DannyTheme_Intro" "/Game/Music_SFXs/Menus/Player_Select_theme.Player_Select_theme" :!type "SoundBase Object Reference") :!label _label))
    (`AudioComponent.SetSound` (`self.MusicIntro`) (`|GetArrayItem` _output_get (`self.SongIndex`)))
    (bind _output_get_2 (set `self.LoopList` (`|MakeArray` "/Game/Music_SFXs/Menus/MainMenu_BGM_Loop.MainMenu_BGM_Loop" "/Game/Music_SFXs/Theme/Arin_Theme_Loop.Arin_Theme_Loop" "/Game/Music_SFXs/Theme/DannyTheme_Loop.DannyTheme_Loop" "/Game/Music_SFXs/Menus/Player_Select_theme.Player_Select_theme" :!type "SoundBase Object Reference")))
    (bind _output (`|GetArrayItem` _output_get_2 (`self.SongIndex`)))
    (`AudioComponent.SetSound` (`self.MusicLoopB`) _output)
    (`AudioComponent.SetSound` (`self.MusicLoop`) _output)
    (`self.MusicStart`)
    (else
      (`self.Stage Start`))))

(event `Stage Start`
  (bind _asggvs_instance (cast `/Game/GeneralNeeds/GGVS_Instance` (`GameplayStatics.GetGameInstance`)))
  (bind _output_get (set `self.P1song` (`/Game/GeneralNeeds/GGVS_Instance.P1Index` _asggvs_instance)))
  (bind _output_get_2 (set `self.P2song` (`/Game/GeneralNeeds/GGVS_Instance.P2Index` _asggvs_instance)))
  (set `self.SongIndex` (`KismetArrayLibrary.Array_Random` (`|MakeArray` _output_get _output_get_2)))
  (goto _label))

(event `MusicStart`
  (add `AudioComponent.OnAudioPlaybackPercent` (`self.MusicIntro`) (delegate `LoopA_%`))
  (`AudioComponent.Play` (`self.MusicIntro`) 0.0)
  (add `AudioComponent.OnAudioPlaybackPercent` (`self.MusicLoop`) (delegate `LoopB%`)))

(event `LoopA_%`
  (params (PlayingSoundWave :type "SoundWave Object Reference") (PlaybackPercent :type "Float (double-precision)"))
  (bind _musicintro (`self.MusicIntro`))
  (if (>= PlaybackPercent 0.993)
    (`/Engine/EditorBlueprintResources/StandardMacros.DoOnce` false :!label _label_2
      (:`Completed`
        (`AudioComponent.FadeOut` _musicintro 0.3 0.0 "Linear")
        (`AudioComponent.FadeIn` (`self.MusicLoop`) 0.2 1.0 0.0 "Linear")
        (`KismetSystemLibrary.Delay` 1.0)
        (`AudioComponent.Stop` _musicintro)
        (set `self.MusicIntro` (`self.MusicLoopB`))))
    (else
      (goto _label_2 :!via `Reset`))))

(event `LoopB%`
  (params (PlayingSoundWave :type "SoundWave Object Reference") (PlaybackPercent :type "Float (double-precision)"))
  (bind _musicloop (`self.MusicLoop`))
  (if (>= PlaybackPercent 0.99)
    (`/Engine/EditorBlueprintResources/StandardMacros.DoOnce` false :!label _label_3
      (:`Completed`
        (`AudioComponent.FadeOut` _musicloop 0.3 0.0 "Linear")
        (`AudioComponent.FadeIn` (`self.MusicIntro`) 0.2 1.0 0.0 "Linear")
        (`KismetSystemLibrary.Delay` 1.0)
        (`AudioComponent.Stop` _musicloop)))
    (else
      (goto _label_3 :!via `Reset`))))

(fn `UserConstructionScript`)