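; Short-lived melee hitbox actor for a fighting game that destroys itself after its active time.
; After a brief delay, its sphere overlap ignores the instigator's side and, once only, sends damage and meter-gain messages to attacker and opponent.
; The hit also triggers hit freeze on both Grump characters.
; Two hit types add extras: one flags Drump success, the other completes a grab by attaching the victim to the attacker's mesh socket.
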(event `self.ReceiveBeginPlay`
  (bind _returnvalue (`self.GetInstigator`))
  (set `self.POwner` (`self.GetOwner`))
  (set `self.PlayerOwner` _returnvalue)
  (set `self.TheSelf` (`self.GetInstigatorController` _returnvalue))
  (`KismetSystemLibrary.Delay` 0.005)
  (`KismetSystemLibrary.Delay` (`self.ActiveTime`))
  (`self.K2_DestroyActor`))

(event `self.Sphere.OnComponentBeginOverlap`
  (params (OverlappedComponent :type "PrimitiveComponent Object Reference") (OtherActor :type "Actor Object Reference") (OtherComp :type "PrimitiveComponent Object Reference") (OtherBodyIndex :type Integer) (bFromSweep :type Boolean) (SweepResult :type "HitResult Structure (by ref)"))
  (`KismetSystemLibrary.Delay` 0.05)
  (if (not (== (`self.GetInstigatorController` OtherActor) (`self.TheSelf`)))
    (set `self.Opponent` OtherActor)
    (`/Engine/EditorBlueprintResources/StandardMacros.DoOnce` false
      (:`Completed`
        (`GameplayStatics.PlaySound2D` (`self.Sound`) 0.3 1.0 0.0 null null)
        (`KismetSystemLibrary.PrintString` (`KismetSystemLibrary.GetDisplayName` OtherActor))
        (message `/Game/GeneralNeeds/Interfaces/Damage_Calc.Damage` (`self.Opponent`) (`KismetMathLibrary.Conv_IntToDouble` (`self.DamageAmount`)) (`self.HitType`) (`self.HitHeight`))
        (message `/Game/GeneralNeeds/Interfaces/MeterGain.MeterGain` (`self.PlayerOwner`) 0.0 (`self.OwnSteamGain`))
        (message `/Game/GeneralNeeds/Interfaces/MeterGain.MeterGain` (`self.Opponent`) (`self.OppSteamGain`) 0.0)
        (`/Engine/EditorBlueprintResources/StandardMacros.DoOnce` false
          (:`Completed`
            (`self.HitFroze`)
            (if (`|EnumEquality` (`self.HitType`) "NewEnumerator3")
              (bind _asbp_grump_parent (cast `/Game/Characters/BP_Grump_Parent` (`self.PlayerOwner`)))
              (set `/Game/Characters/BP_Grump_Parent.DrumpSuccess` true _asbp_grump_parent)
              (elif (`|EnumEquality` (`self.HitType`) "NewEnumerator8")
                (`KismetSystemLibrary.PrintString` "Grab SUcceeded")
                (bind _asbp_grump_parent_2 (cast `/Game/Characters/BP_Grump_Parent` (`self.PlayerOwner`)))
                (set `/Game/Characters/BP_Grump_Parent.AttemptingGrab` false _asbp_grump_parent_2)
                (set `/Game/Characters/BP_Grump_Parent.GrabSuccess` true _asbp_grump_parent_2)
                (bind _asbp_grump_parent_3 (cast `/Game/Characters/BP_Grump_Parent` (`self.Opponent`)))
                (`/Game/Characters/BP_Grump_Parent.GrabbedCollisionsOff` _asbp_grump_parent_3)
                (`self.K2_AttachToComponent` _asbp_grump_parent_3 (`Character.Mesh` _asbp_grump_parent_2) (`self.GrabSocket`) "SnapToTarget" "SnapToTarget" "KeepWorld" true)))))))))

(event `HitFroze`
  (bind _hittype (`self.HitType`))
  ;[1 1 1] HitFreeze Per Hit
  (bind _asbp_grump_parent (cast `/Game/Characters/BP_Grump_Parent` (`self.PlayerOwner`)))
  (bind _asbp_grump_parent_2 (cast `/Game/Characters/BP_Grump_Parent` (`self.Opponent`)))
  (`/Game/Characters/BP_Grump_Parent.HitFroze` _asbp_grump_parent _hittype)
  (`/Game/Characters/BP_Grump_Parent.HitFroze` _asbp_grump_parent_2 _hittype))

(fn `UserConstructionScript`)